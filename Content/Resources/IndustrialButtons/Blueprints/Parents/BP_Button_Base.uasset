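; Parent Blueprint for industrial button props that sets up the look of the button's base.
; The Construction Script picks the base mesh from an array using the Basetype value.
; DirtyColorset switches between the preset MI_Bases material and a dynamic instance of MI_BasesClean tinted through its Basecolor parameter.
; The event graph holds only disabled placeholder events, so this class adds no runtime behavior.
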(fn `UserConstructionScript`
  (`StaticMeshComponent.SetStaticMesh` (`self.SM_Base`) (`|GetArrayItem` (`self.Meshes`) (`KismetMathLibrary.Conv_ByteToInt` (`self.Basetype`))))
  (if (`self.DirtyColorset`)
    (`PrimitiveComponent.SetMaterial` (`self.SM_Base`) 0 "/Game/Resources/IndustrialButtons/Materials/Instances/MI_Bases.MI_Bases")
    (else
      (bind _returnvalue (`PrimitiveComponent.CreateDynamicMaterialInstance` (`self.SM_Base`) 0 "/Game/Resources/IndustrialButtons/Materials/Instances/MI_BasesClean.MI_BasesClean" "None"))
      (`PrimitiveComponent.SetMaterial` (`self.SM_Base`) 0 _returnvalue)
      (`MaterialInstanceDynamic.SetVectorParameterValue` _returnvalue "Basecolor" (`self.Color`)))))