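; BP_Buttons_Double is a parent Blueprint for an industrial double button with separate on and off button meshes and an optional base.
; Its Construction Script sets base visibility from ShowBase, then uses the On flag to offset the active button by PressedOffset along Z and set the other's relative location to zero.
; BeginPlay is empty, so the file only sets the visual state at construction and has no runtime interaction.
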(event `self.ReceiveBeginPlay`)

(fn `UserConstructionScript`
  (`SceneComponent.SetVisibility` (`self.SM_Base`) (`self.ShowBase`) false)
  (if (`self.On`)
    (`SceneComponent.K2_AddLocalOffset` (`self.SM_Button_On`) (`KismetMathLibrary.MakeVector` 0.0 0.0 (`self.Pressed_Offset`)) false false)
    (`SceneComponent.K2_SetRelativeLocation` (`self.SM_Button_Off`) (0.0 0.0 0.0) false false)
    (else
      (`SceneComponent.K2_AddLocalOffset` (`self.SM_Button_Off`) (`KismetMathLibrary.MakeVector` 0.0 0.0 (`self.Pressed_Offset`)) false false)
      (`SceneComponent.K2_SetRelativeLocation` (`self.SM_Button_On`) (0.0 0.0 0.0) false false))))