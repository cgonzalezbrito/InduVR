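; BP_Button_Single_Colorchange is a parent Blueprint for industrial single buttons with a configurable color.
; Its construction script runs the parent script, then creates a dynamic material instance from slot 0 of the Button component.
; It writes ButtonColor to the vector parameter named by ColorParameter on that instance.
; The event graph contains only disabled default events, so this Blueprint adds no runtime logic.
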(fn `UserConstructionScript`
  (bind _button (`self.Button`))
  (`parent.UserConstructionScript`)
  (bind _returnvalue (`PrimitiveComponent.CreateDynamicMaterialInstance` _button 0 (`PrimitiveComponent.GetMaterial` _button 0) "None"))
  (`MaterialInstanceDynamic.SetVectorParameterValue` _returnvalue (`self.Color_Parameter`) (`self.ButtonColor`)))