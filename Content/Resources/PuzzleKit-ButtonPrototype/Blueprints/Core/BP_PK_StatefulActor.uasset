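; BP_PK_StatefulActor is a puzzle kit actor that owns an iterative state component and exposes its current state.
; Action requests are forwarded to the component only with authority.
; Observer change and failure events are filtered to those sent by its own component, then passed to own-state handlers.
; Those handlers are empty hooks, not meant to be called directly by other actors.
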(event `PK_DoAction`
  (params (Action :type "/Game/Resources/PuzzleKit-ButtonPrototype/Blueprints/Core/Enums/EPK_StateAction Enum" :default "NewEnumerator9") (Instigator :type "Actor Object Reference"))
  ;[1 1 1] Calls appropriate action on StateComponent
  (`/Engine/EditorBlueprintResources/ActorMacros.Switch Has Authority`
    (:`Authority`
      (bind _iterativestatecomp (`self.IterativeStateComp`)
        (:`then`
          (`/Game/Resources/PuzzleKit-ButtonPrototype/Blueprints/Core/BP_PK_IterativeStateComponent.PK_DoAction` _iterativestatecomp Action Instigator))
        (:`else`)))))

(event `PK_HandleOwnStateChanged`
  (params (NewStateId :type Byte) (Args :type "/Game/Resources/PuzzleKit-ButtonPrototype/Blueprints/Core/Structs/FPKStateChangeArgs Structure"))
  ;[0.5833 1 0.6334] Called by StateComponent, on state change success. Should never be called directly by another actor
)

(event `PK_HandleOwnChangeFailure`
  (params (Args :type "/Game/Resources/PuzzleKit-ButtonPrototype/Blueprints/Core/Structs/FPKStateChangeArgs Structure") (FailReason :type "/Game/Resources/PuzzleKit-ButtonPrototype/Blueprints/Core/Enums/EPK_FailReason Enum" :default "NewEnumerator3"))
  ;[1 0.5573 0.5573] Called by StateComponent, on state change failure. Should never be called directly by another actor
)

(event `/Game/Resources/PuzzleKit-ButtonPrototype/Blueprints/Core/BPI_PK_ObserverActor.PK_HandleStateChanged`
  (params (ChangeArgs :type "/Game/Resources/PuzzleKit-ButtonPrototype/Blueprints/Core/Structs/FPKStateChangeArgs Structure"))
  (bind _iterativestatecomp (`self.IterativeStateComp`))
  (bind (_stateinfo _stateid _bisvalid) (`/Game/Resources/PuzzleKit-ButtonPrototype/Blueprints/Core/BP_PK_IterativeStateComponent.GetState` _iterativestatecomp))
  ;[1 1 1] PK_ObserverActor events
  ;;[0.5833 1 0.6334] Handle change events, if they come from owned state component
  (if (== (`.Sender_73_060B4A234DECD89FFF920A833D98B38C` (break `/Game/Resources/PuzzleKit-ButtonPrototype/Blueprints/Core/Structs/FPKStateChangeArgs` ChangeArgs)) _iterativestatecomp)
    (if _bisvalid
      (`self.PK_HandleOwnStateChanged` _stateid ChangeArgs))))

(event `/Game/Resources/PuzzleKit-ButtonPrototype/Blueprints/Core/BPI_PK_ObserverActor.PK_HandleChangeFailure`
  (params (ChangeArgs :type "/Game/Resources/PuzzleKit-ButtonPrototype/Blueprints/Core/Structs/FPKStateChangeArgs Structure") (FailReason :type "/Game/Resources/PuzzleKit-ButtonPrototype/Blueprints/Core/Enums/EPK_FailReason Enum" :default "NewEnumerator3"))
  ;[1 1 1] PK_ObserverActor events
  ;;[1 0.5573 0.5573] Handle failure events, if they come from the owned state component
  (if (== (`.Sender_73_060B4A234DECD89FFF920A833D98B38C` (break `/Game/Resources/PuzzleKit-ButtonPrototype/Blueprints/Core/Structs/FPKStateChangeArgs` ChangeArgs)) (`self.IterativeStateComp`))
    (`self.PK_HandleOwnChangeFailure` ChangeArgs FailReason)))

(fn `GetState`
  (returns (StateInfo :type String))
  (bind _iterativestatecomp (`self.IterativeStateComp`)
    (:`then`
      (bind (_stateinfo _stateid _bisvalid) (`/Game/Resources/PuzzleKit-ButtonPrototype/Blueprints/Core/BP_PK_IterativeStateComponent.GetState` _iterativestatecomp))
      (if _bisvalid
        (return _stateinfo)))
    (:`else`)))

(fn `UserConstructionScript`)